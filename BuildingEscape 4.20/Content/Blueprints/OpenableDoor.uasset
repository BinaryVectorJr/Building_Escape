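; A door actor that swings open and closed in response to OnOpen and OnClose events from its OpenDoor component.
; The DoorSwing timeline plays forward to open and in reverse to close, driving the yaw from its OpenAngle track.
; That yaw is combined with the rotation stored at BeginPlay, so the door works facing any direction.
; An event track on the timeline plays a lock sound at the door's location.
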(event `self.ReceiveBeginPlay`
  ;[1 1 1] Store the initial rotation of the door when Play is pressed
  (set `self.InitialRotation` (`self.K2_GetActorRotation`)))

(event `self.OpenDoor.OnOpen`
  ;[1 1 1] Door open-close "animation" --> now the door can face any direction
  (bind (_direction _openangle) (`Timeline|DoorSwing` :!label _label)
    (:`Update`
      _)
    (:`LockingSound`
      (`GameplayStatics.PlaySoundAtLocation` "/Game/Audio/door_lock.door_lock" (`self.K2_GetActorLocation`) (struct) 1.0 1.0 0.0 null null null)))
  (`self.K2_SetActorRotation` (`KismetMathLibrary.ComposeRotators` (`KismetMathLibrary.MakeRotator` 0.0 0.0 _openangle) (`self.InitialRotation`))))

(event `self.OpenDoor.OnClose`
  ;[1 1 1] Door open-close "animation" --> now the door can face any direction
  (goto _label :!via `Reverse`))

(fn `UserConstructionScript`)